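; Lantern pickup actor that gives the first-person character the lamp when it enters the Box trigger.
; On overlap it sets LampObtained on the character, casts to MainGameInstance, adds a HUD widget to the viewport and destroys itself.
; On BeginPlay it removes itself if the game instance's LightActive is set, meant for deaths on level one.
; The nodes setting LightActive and GotLamp are disconnected and never run.
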(event `self.Box.OnComponentBeginOverlap`
  (params (OverlappedComponent :type "PrimitiveComponent Object Reference") (OtherActor :type "Actor Object Reference") (OtherComp :type "PrimitiveComponent Object Reference") (OtherBodyIndex :type Integer) (bFromSweep :type Boolean) (SweepResult :type "HitResult Structure (by ref)"))
  ;[1 1 1] Pick up lantern
  (bind _asbp_first_person_character (cast `/Game/ScaryGame/Blueprints/BP_FirstPersonCharacter` OtherActor))
  (set `/Game/ScaryGame/Blueprints/BP_FirstPersonCharacter.lampObtained` true _asbp_first_person_character)
  (bind _asmain_game_instance (cast `/Game/ScaryGame/Blueprints/MainGameInstance` (`GameplayStatics.GetGameInstance`)))
  (bind _returnvalue (`|CreateWidget` "/Game/ScaryGame/UI/HUD.HUD_C"))
  (`UserWidget.AddToViewport` _returnvalue 0)
  (`self.K2_DestroyActor`))

(event `self.ReceiveBeginPlay`
  ;[1 1 1] For if player dies on lv one
  (bind _asmain_game_instance (cast `/Game/ScaryGame/Blueprints/MainGameInstance` (`GameplayStatics.GetGameInstance`)))
  (if (`/Game/ScaryGame/Blueprints/MainGameInstance.LightActive` _asmain_game_instance)
    (`self.K2_DestroyActor`)))

(fn `UserConstructionScript`)